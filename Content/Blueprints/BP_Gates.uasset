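; BP_Gates is a goal actor that awards a point and resets the ball when a BP_BallActor enters its Box trigger.
; On overlap it increments the score of the team selected by Is1Player in MainGameState, which it caches at BeginPlay.
; It then calls a server-named event that destroys the ball and spawns a fresh one at a fixed location.
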(event OnComponentBeginOverlap(Box)
  (params (OverlappedComponent :type Primitive%20Component%20Object%20Reference) (OtherActor :type Actor%20Object%20Reference) (OtherComp :type Primitive%20Component%20Object%20Reference) (OtherBodyIndex :type Integer) (bFromSweep :type Boolean) (SweepResult :type Hit%20Result%20Structure%20%28by%20ref%29))
  (bind _is1player_ (Variables|Default|Getis1Player?))
  (bind _as_main_game_state (Variables|Default|GetAs%20Main%20Game%20State))
  (bind _asbp_ball_actor (Utilities|Casting|CastToBP_BallActor OtherActor))
  (bind _returnvalue (Class|MainGameState|GetTeamScore _as_main_game_state _is1player_))
  (Class|MainGameState|SetTeamScore _as_main_game_state _is1player_ (+ _returnvalue 1))
  (CallFunction|ServerHandleBallAfterScore "/Game/Blueprints/BP_BallActor.BP_BallActor_C" "0.000000,0.000000,-300.000000" _asbp_ball_actor))

(event Custom|Server_HandleBallAfterScore
  (params (Class :type Actor%20Class%20Reference) (Spawn%20Transform%20Location :type Vector) (Target :type Actor%20Object%20Reference))
  (Actor|DestroyActor Target)
  (Game|SpawnActorfromClass Class (Math|Transform|MakeTransform Spawn%20Transform%20Location "0, 0, 0" "1.000000,1.000000,1.000000") "Undefined" "MultiplyWithRoot" 0 0))

(event EventBeginPlay
  (bind _asmain_game_state (Utilities|Casting|CastToMainGameState (Game|GetGameState)))
  (Variables|Default|SetAs%20Main%20Game%20State _asmain_game_state))

(fn ConstructionScript)